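; BP_WallCreator switches the state of BP_WallManager walls according to whether they stand between the camera and the player.
; BeginPlay caches the PlayerCamera, CharacterController and all wall actors.
; Each Tick repeats a horizontal Visibility trace at player height from the camera's XY, ignoring previous hits until it reaches the player or hits the iteration cap.
; Walls hit receive ChangeStateEvent(false); all others receive true.
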(event EventBeginPlay
  (bind _outactors (Actor|GetAllActorsOfClass "/Script/KaijuGJ2022.PlayerCamera"))
  (for _array_element _outactors
    (Variables|Default|SetCamera _array_element))
  (bind _outactors_2 (Actor|GetAllActorsOfClass "/Script/KaijuGJ2022.CharacterController"))
  (for _array_element_2 _outactors_2
    (Variables|Default|SetPlayer _array_element_2)
    (bind _outactors_3 (Actor|GetAllActorsOfClass "/Game/blueprints/BP_WallManager.BP_WallManager_C"))
    (Variables|Default|SetWalls _outactors_3)))

(event EventTick
  (params (DeltaSeconds :type Float%20%28single-precision%29))
  (bind _player (Variables|Default|GetPlayer))
  (bind _camera (Variables|Default|GetCamera))
  (bind _returnvalue (Transformation|GetActorLocation _player))
  (bind _returnvalue_2 (Actor|GetComponentsByClass _camera "/Script/Engine.CameraComponent"))
  (bind _output (Utilities|Array|Get(acopy) _returnvalue_2))
  (bind _returnvalue_3 (Transformation|GetWorldLocation _output))
  (bind (_x _y) (Math|Vector|BreakVector _returnvalue_3))
  (Variables|Default|SetHitActors (Utilities|Array|MakeArray 0))
  (Utilities|FlowControl|ForLoopwithBreak 0 10 :!label _label
    (:LoopBody
      (bind _outhit (Collision|LineTraceByChannel (Math|Vector|MakeVector _x _y (.Z (Math|Vector|BreakVector _returnvalue))) _returnvalue "TraceTypeQuery1" false (Variables|Default|GetHitActors) "None"))
      (if (== (.HitActor (Collision|BreakHitResult _outhit)) (Variables|Default|GetPlayer))
        (goto _label Break)
        (else
          (Utilities|Array|Add (Variables|Default|GetHitActors) (.HitActor (Collision|BreakHitResult _outhit))))))
    (:Completed
      (for _array_element (Variables|Default|GetWalls)
        (if (== (Utilities|Array|FindItem (Variables|Default|GetHitActors) _array_element) -1)
          (bind _asbp_wall_manager (Utilities|Casting|CastToBP_WallManager _array_element))
          (Default|ChangeStateEvent _asbp_wall_manager true)
          (else
            (bind _asbp_wall_manager_2 (Utilities|Casting|CastToBP_WallManager _array_element))
            (Default|ChangeStateEvent _asbp_wall_manager_2 false)))))))

(fn ConstructionScript)