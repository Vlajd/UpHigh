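; BP_Hand_Mesh is a hand actor that grabs and kills the player on overlap.
; BeginPlay caches its anim instance and the first BP_CharacterController, and binds SetOverlapping to the anim blueprint to re-enable the Overlapper.
; An overlap disables further overlaps, triggers the animation and calls PlayerDeath.
; A while loop, with no delay, then snaps the player to the hand's grab socket while MIsSummoning is true.
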(event Custom|Set%20Overlapping
  (Variables|/Script/Engine.PrimitiveComponent|SetbGenerateOverlapEvents (Variables|Default|GetOverlapper) true))

(event EventBeginPlay
  (bind _asbp_hand_mesh_anim (Utilities|Casting|CastToBP_Hand_Mesh_Anim (Components|SkeletalMesh|GetAnimInstance (Variables|Default|GetHand)))
    (:then
      (Variables|Default|SetBP_Hand_Mesh_Anim _asbp_hand_mesh_anim))
    (:CastFailed
      (Development|PrintString "HelloBP_Hand_Mesh_Anim Cast Failed")))
  (Variables|/Script/Engine.PrimitiveComponent|SetbGenerateOverlapEvents (Variables|Default|GetOverlapper) true)
  (bind _assample_player_controller (Utilities|Casting|CastToSamplePlayerController (Game|GetPlayerController 0))
    (:then
      (Variables|Default|SetSamplePlayerController _assample_player_controller)
      (bind _outactors (Actor|GetAllActorsOfClass "/Game/blueprints/BP_CharacterController.BP_CharacterController_C"))
      (Variables|Default|SetBP_CharacterController (Utilities|Array|Get(acopy) _outactors))
      (EventDispatchers|BindEventtoSetOverlapping (Variables|Default|GetBP_Hand_Mesh_Anim) (delegate Custom|Set%20Overlapping)))
    (:CastFailed
      (Development|PrintString "SamplePlayerController Cast Failed"))))

(event Collision|EventActorBeginOverlap
  (params (OtherActor :type Actor%20Object%20Reference))
  (bind _bp_charactercontroller (Variables|Default|GetBP_CharacterController))
  (Variables|/Script/Engine.PrimitiveComponent|SetbGenerateOverlapEvents (Variables|Default|GetOverlapper) false)
  (Variables|/Game/blueprints/BP_Hand/BP_Hand_Mesh_Anim.BP_Hand_Mesh_Anim_C|SetPlayAnim (Variables|Default|GetBP_Hand_Mesh_Anim) true)
  (Class|CharacterController|PlayerDeath _bp_charactercontroller)
  (while (Variables|/Script/KaijuGJ2022.CharacterController|Getm_IsSummoning _bp_charactercontroller)
    (Transformation|SetActorLocation _bp_charactercontroller (Transformation|GetSocketLocation (Variables|Default|GetHand) "Socket_PlayerGrabPos") false false)))

(fn ConstructionScript)