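; BP_Hand_Music is a hand hazard that alternates between up and down on a timed rhythm and kills the player on overlap.
; Tick uses a Delay of Bps to flip IsDown on the hand's anim instance, enabling overlap events only while down.
; On overlap it calls PlayerDeath, plays death and window-breaking sounds, then loops teleporting the player to the grab socket while MIsSummoning holds.
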(event EventBeginPlay
  (bind _asbp_sample_player_controller (Utilities|Casting|CastToBP_SamplePlayerController (Game|GetPlayerController 0))
    (:then
      (Variables|Default|SetSamplePlayerController _asbp_sample_player_controller))
    (:CastFailed
      (Development|PrintString "SamplePlayerController Cast Failed")))
  (bind _outactors (Actor|GetAllActorsOfClass "/Game/blueprints/BP_CharacterController.BP_CharacterController_C"))
  (Variables|Default|SetBP_CharacterController (Utilities|Array|Get(acopy) _outactors))
  (bind _asbp_hand_music_anim (Utilities|Casting|CastToBP_Hand_Music_Anim (Components|SkeletalMesh|GetAnimInstance (Variables|Default|GetHand)))
    (:then
      (Variables|Default|SetBP_Hand_Music_Anim _asbp_hand_music_anim))
    (:CastFailed
      (Development|PrintString "BP_Hand_Music_Anim cast failed"))))

(event EventTick
  (params (DeltaSeconds :type Float%20%28single-precision%29))
  (bind _bp_hand_music_anim (Variables|Default|GetBP_Hand_Music_Anim))
  (Utilities|FlowControl|Delay (Variables|Default|Getbps))
  (bind _output_get (Variables|/Game/blueprints/BP_Hand/BP_Hand_Music_Anim.BP_Hand_Music_Anim_C|SetIsDown _bp_hand_music_anim (not (Variables|/Game/blueprints/BP_Hand/BP_Hand_Music_Anim.BP_Hand_Music_Anim_C|GetIsDown _bp_hand_music_anim))))
  (Variables|/Script/Engine.PrimitiveComponent|SetbGenerateOverlapEvents (Variables|Default|GetOverlapper) _output_get))

(event Collision|EventActorBeginOverlap
  (params (OtherActor :type Actor%20Object%20Reference))
  (bind _hand (Variables|Default|GetHand))
  (bind _bp_charactercontroller (Variables|Default|GetBP_CharacterController))
  (bind _returnvalue (Transformation|GetSocketLocation _hand "Socket_PlayerGrabPos"))
  (Variables|/Script/Engine.PrimitiveComponent|SetbGenerateOverlapEvents (Variables|Default|GetOverlapper) false)
  (Class|CharacterController|PlayerDeath _bp_charactercontroller)
  (Audio|PlaySound2D "/Game/audio/envSounds/Death_Sound_Cue.Death_Sound_Cue" 1.0 1.0 0.0 0 0)
  (Audio|PlaySoundatLocation "/Game/audio/envSounds/window_breaking_cue.window_breaking_cue" (Transformation|GetActorLocation) "0, 0, 0" 1.0 1.0 0.0 0 0 0)
  (while (Variables|/Script/KaijuGJ2022.CharacterController|Getm_IsSummoning _bp_charactercontroller)
    (Transformation|SetActorLocation _bp_charactercontroller _returnvalue false false)
    (Audio|PlaySoundatLocation "/Game/audio/envSounds/window_breaking_cue.window_breaking_cue" _returnvalue "0, 0, 0" 1.0 1.0 0.0 0 0 0)
    (Audio|PlaySound2D "/Game/audio/envSounds/Death_Sound_Cue.Death_Sound_Cue" 1.0 1.0 0.0 0 0)))

(fn ConstructionScript)