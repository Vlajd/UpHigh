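; BP_MainMenuBase sets up the main menu and starts its theme music when play begins.
; It adds the BP_MainMenu widget to the viewport, switches the player to UI-only input and shows the mouse cursor.
; If BP_SampleGameInstance holds no MenuTheme yet, it creates a 2D sound that persists across level transitions, stores it there and plays it, avoiding a duplicate track on later visits.
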(event EventBeginPlay
  (bind _returnvalue (Game|GetPlayerController 0))
  (bind _returnvalue_2 (UserInterface|CreateWidget "/Game/blueprints/menus/BP_MainMenu.BP_MainMenu_C"))
  (UserInterface|Viewport|AddtoViewport _returnvalue_2 0)
  (Input|SetInputModeUIOnly _returnvalue 0 "DoNotLock")
  (Variables|/Script/Engine.PlayerController|SetbShowMouseCursor _returnvalue true)
  (bind _asbp_sample_game_instance (Utilities|Casting|CastToBP_SampleGameInstance (Game|GetGameInstance)))
  (if (== (Variables|/Game/blueprints/BP_SampleGameInstance.BP_SampleGameInstance_C|GetMenuTheme _asbp_sample_game_instance) 0)
    (bind _returnvalue_3 (Audio|CreateSound2D "/Game/audio/envSounds/MenuTheme_Cue.MenuTheme_Cue" 1.0 1.0 0.0 0 true))
    (bind _output_get (Variables|/Game/blueprints/BP_SampleGameInstance.BP_SampleGameInstance_C|SetMenuTheme _asbp_sample_game_instance _returnvalue_3))
    (Audio|Components|Audio|Play _output_get 0.0)))

(fn ConstructionScript)