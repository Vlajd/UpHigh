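; LevelObject is a mesh actor tied to a level number that removes itself once the game moves past that level.
; Its construction script applies one ObjectMesh to both the visible Mesh and a ShadowCollisionMesh component.
; LevelChangeEvent compares MyLevel with the incoming NewLevel and, when MyLevel is lower, prints the root component's display name and destroys the actor.
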(event Custom|LevelChange%20Event
  (params (NewLevel :type Integer))
  (if (< (Variables|Default|GetMyLevel) NewLevel)
    (Development|PrintString (Utilities|GetDisplayName (Variables|Default|GetDefaultSceneRoot)))
    (Actor|DestroyActor)))

(fn ConstructionScript
  (bind _objectmesh (Variables|Default|GetObjectMesh))
  (Components|StaticMesh|SetStaticMesh (Variables|Default|GetMesh) _objectmesh)
  (Components|StaticMesh|SetStaticMesh (Variables|Default|GetShadowCollisionMesh) _objectmesh))