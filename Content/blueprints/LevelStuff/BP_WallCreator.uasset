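; BP_WallCreator switches the state of WallObject actors that stand between the player camera and the CharacterController actor, apparently to keep the player in view.
; Each tick it repeats a visibility line trace from camera to player, adding each hit to the ignore list until it reaches the player or the loop limit.
; Walls in that hit list receive StateChangeEvent(false); all others receive true, as does every wall while CurrentlyAnimating is set.
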(event EventBeginPlay
  (bind _asbp_player_camera (Utilities|Casting|CastToBP_PlayerCamera (Game|Player|GetPlayerPawn 0)))
  (Variables|Default|SetCamera (Utilities|Array|Get(acopy) (Actor|GetComponentsByClass _asbp_player_camera "/Script/Engine.CameraComponent")))
  (bind _outactors (Actor|GetAllActorsOfClass "/Script/KaijuGJ2022.CharacterController"))
  (for _array_element _outactors
    (Variables|Default|SetPlayer _array_element)))

(event EventTick
  (params (DeltaSeconds :type Float%20%28single-precision%29))
  (bind _outactors (Actor|GetAllActorsOfClass "/Game/blueprints/LevelStuff/WallObject.WallObject_C"))
  (Variables|Default|SetWalls _outactors)
  (Variables|Default|SetHitActors (Utilities|Array|MakeArray 0))
  (Utilities|FlowControl|ForLoopwithBreak 0 10 :!label _label
    (:LoopBody
      (bind _outhit (Collision|LineTraceByChannel (Transformation|GetWorldLocation (Variables|Default|GetCamera)) (Transformation|GetActorLocation (Variables|Default|GetPlayer)) "TraceTypeQuery1" false (Variables|Default|GetHitActors) "None"))
      (if (== (.HitActor (Collision|BreakHitResult _outhit)) (Variables|Default|GetPlayer))
        (goto _label Break)
        (else
          (Utilities|Array|Add (Variables|Default|GetHitActors) (.HitActor (Collision|BreakHitResult _outhit))))))
    (:Completed
      (for _array_element (Variables|Default|GetWalls)
        (if (or (== (Utilities|Array|FindItem (Variables|Default|GetHitActors) _array_element) -1) (Variables|Default|Getcurrently%20animating))
          (bind _aswall_object (Utilities|Casting|CastToWallObject _array_element))
          (Default|StateChangeEvent _aswall_object true)
          (else
            (bind _aswall_object_2 (Utilities|Casting|CastToWallObject _array_element))
            (Default|StateChangeEvent _aswall_object_2 false)))))))

(fn ConstructionScript)