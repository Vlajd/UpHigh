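; LevelStairs is a stairs actor that shows or hides itself according to the active level.
; The construction script applies one ObjectMesh to both the visible Mesh and a ShadowCollisionMesh.
; LevelChangeEvent compares the new level to MyLevel, then toggles visibility on the root and its children and switches both meshes between QueryAndPhysics and no collision.
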(event Custom|LevelChange%20Event
  (params (NewLevel :type Integer))
  (bind _defaultsceneroot (Variables|Default|GetDefaultSceneRoot))
  (bind _mesh (Variables|Default|GetMesh))
  (bind _shadowcollisionmesh (Variables|Default|GetShadowCollisionMesh))
  (if (!= NewLevel (Variables|Default|GetMyLevel))
    (Rendering|SetVisibility _defaultsceneroot false true)
    (Collision|SetCollisionEnabled _mesh "NoCollision")
    (Collision|SetCollisionEnabled _shadowcollisionmesh "NoCollision")
    (else
      (Rendering|SetVisibility _defaultsceneroot true true)
      (Collision|SetCollisionEnabled _mesh "QueryAndPhysics")
      (Collision|SetCollisionEnabled _shadowcollisionmesh "QueryAndPhysics"))))

(fn ConstructionScript
  (bind _objectmesh (Variables|Default|GetObjectMesh))
  (Components|StaticMesh|SetStaticMesh (Variables|Default|GetMesh) _objectmesh)
  (Components|StaticMesh|SetStaticMesh (Variables|Default|GetShadowCollisionMesh) _objectmesh))