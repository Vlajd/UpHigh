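; BP_Eye is a watching-eye hazard that kills the player when they stay in its line of sight.
; Each Tick it traces from the eye to the first BP_CharacterController actor found, showing a cable as a gaze beam when unblocked.
; While sight is clear, the eye and cable end lerp toward the player.
; After a TimeTillPlayerDead delay, a still-clear trace calls PlayerDeath and plays the death sound.
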(event EventBeginPlay
  (bind _outactors (Actor|GetAllActorsOfClass "/Game/blueprints/BP_CharacterController.BP_CharacterController_C"))
  (Variables|Default|SetBP_CharacterController (Utilities|Array|Get(acopy) _outactors))
  (bind _asbp_sample_player_controller (Utilities|Casting|CastToBP_SamplePlayerController (Game|GetPlayerController 0))
    (:then
      (Variables|Default|SetBP_SamplePlayerController _asbp_sample_player_controller))
    (:CastFailed
      (Development|PrintString "BP_SamplePlayerController Cast Failed"))))

(event EventTick
  (params (DeltaSeconds :type Float%20%28single-precision%29))
  (bind _returnvalue (Math|Rotator|MakeRotator 0.0 -5.0 87.0))
  (bind _sphere (Variables|Default|GetSphere))
  (bind _bp_charactercontroller (Variables|Default|GetBP_CharacterController))
  (bind _eyeorigin (Variables|Default|GetEyeOrigin))
  (bind _eyerotspeed (Variables|Script|GetEyeRotSpeed))
  (bind _cable (Variables|Default|GetCable))
  (bind _returnvalue_2 (Transformation|GetWorldLocation _eyeorigin))
  (bind _returnvalue_3 (Transformation|GetActorLocation _bp_charactercontroller))
  (bind _relativerotation (Variables|/Script/Engine.SceneComponent|GetRelativeRotation _eyeorigin))
  (bind _relativerotation_2 (Variables|/Script/Engine.SceneComponent|GetRelativeRotation _sphere))
  (bind _returnvalue_4 (Math|Rotator|FindLookatRotation _returnvalue_2 _returnvalue_3))
  (bind _returnvalue_5 (Math|Rotator|CombineRotators _returnvalue_4 _returnvalue))
  (bind _returnvalue_6 (Math|Rotator|Lerp(Rotator) _returnvalue_5 _relativerotation _eyerotspeed true))
  (bind (_outhit _returnvalue_7) (Collision|LineTraceByChannel _returnvalue_2 _returnvalue_3 "TraceTypeQuery1" true 0 "None" true "(R=0.000000,G=0.000000,B=0.000000,A=0.000000)" "(R=0.300000,G=0.004800,B=0.000000,A=1.000000)"))
  (Rendering|SetVisibility _cable (Math|Boolean|NANDBoolean _returnvalue_7 (.bBlockingHit (Collision|BreakHitResult _outhit))) false)
  (if (Math|Boolean|NANDBoolean _returnvalue_7 (.bBlockingHit (Collision|BreakHitResult _outhit)))
    (Transformation|SetRelativeRotation _eyeorigin (Math|Rotator|MakeRotator (+ (.roll _returnvalue_6) (* (.roll _relativerotation_2) 0.5)) (+ (.pitch _returnvalue_6) (* (.pitch _relativerotation_2) 0.5)) (+ (.yaw _returnvalue_6) (* (.yaw _relativerotation_2) 0.5))) false false)
    (Variables|/Script/CableComponent.CableComponent|SetEndLocation _cable (Math|Vector|Lerp(Vector) (Variables|/Script/CableComponent.CableComponent|GetEndLocation _cable) (- _returnvalue_3 (Transformation|GetWorldLocation (Variables|Default|GetSphere))) (Variables|Script|GetEyeRotSpeed)))
    (Utilities|FlowControl|Delay (Variables|Script|GetTimeTillPlayerDead))
    (if (Math|Boolean|NANDBoolean _returnvalue_7 (.bBlockingHit (Collision|BreakHitResult _outhit)))
      (Class|CharacterController|PlayerDeath (Variables|Default|GetBP_CharacterController))
      (Audio|PlaySound2D "/Game/audio/envSounds/Death_Sound_Cue.Death_Sound_Cue" 1.0 1.0 0.0 0 0))))

(fn ConstructionScript)