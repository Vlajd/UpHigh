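; Player character Blueprint that links movement and use actions to its animation Blueprint and toggles the pause menu.
; Tick feeds velocity to BP_Character_Anim and re-enables SamplePlayerController input whenever the anim instance is not using.
; A use event passes the use type to the anim instance, flags it as using and disables input.
; A FlipFlop alternately opens and removes the pause widget, toggling game pause and cursor visibility.
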(event EventBeginPlay
  (bind _assample_player_controller (Utilities|Casting|CastToSamplePlayerController (Class|GameplayStatics|GetPlayerControllerfromID))))

(event EventTick
  (params (DeltaSeconds :type Float%20%28single-precision%29))
  (bind _returnvalue (Class|CharacterController|GetCurrentVelocity))
  (bind _asbp_character_anim (Utilities|Casting|CastToBP_Character_Anim (Components|SkeletalMesh|GetAnimInstance (Variables|Default|GetCharacterSkeletalMesh)))
    (:then
      (Class|CharacterAnimation|SetIsMoving _asbp_character_anim _returnvalue)
      (if (not (Variables|/Game/blueprints/BP_Character_Anim.BP_Character_Anim_C|GetIsUsing _asbp_character_anim))
        (Class|SamplePlayerController|SetPlayerInputTrue (stale EventBeginPlay _assample_player_controller))))
    (:CastFailed
      (Development|PrintString "Cast Failed"))))

(event EventShowPauseMenu
  (bind _returnvalue (Game|GetPlayerController 0))
  (Utilities|FlowControl|FlipFlop
    (:A
      (bind _returnvalue_2 (UserInterface|CreateWidget "/Game/blueprints/BP_PauseMenu.BP_PauseMenu_C"))
      (UserInterface|Viewport|AddtoViewport _returnvalue_2 0)
      (Game|SetGamePaused true)
      (Variables|/Script/Engine.PlayerController|SetbShowMouseCursor _returnvalue true))
    (:B
      (Widget|RemovefromParent _returnvalue_2)
      (Game|SetGamePaused false)
      (Variables|/Script/Engine.PlayerController|SetbShowMouseCursor _returnvalue false))))

(event EventUFUNCTIONCallSetIsUsing
  (params (useType :type Integer))
  (Variables|/Game/blueprints/BP_Character_Anim.BP_Character_Anim_C|SetUseTypeAnim (stale EventTick _asbp_character_anim) useType)
  (Variables|/Game/blueprints/BP_Character_Anim.BP_Character_Anim_C|SetIsUsing (stale EventTick _asbp_character_anim) true)
  (Class|SamplePlayerController|SetPlayerInputFalse (stale EventBeginPlay _assample_player_controller)))

(fn ConstructionScript)