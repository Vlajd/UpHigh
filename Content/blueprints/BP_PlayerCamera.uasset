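; BP_PlayerCamera is an orbit-style player camera with yaw, clamped pitch and smoothed zoom.
; Rotation events turn the RotOrigin pivot, which BeginPlay places at a fixed relative offset.
; The zoom event moves ZoomTarget along negative X within distance limits, and Tick lerps the Camera toward it by DeltaSeconds times ZoomSpeed.
; The construction script hard-sets the offset, pitch limits, zoom limits and speed.
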(event EventBeginPlay
  (Transformation|SetRelativeLocation (Variables|Default|GetRotOrigin) (Variables|Default|GetCameraOriginSpawnLocation) false false)
  (Transformation|SetRelativeTransform (Variables|Default|GetZoomTarget) (Transformation|GetRelativeTransform (Variables|Default|GetCamera)) false false))

(event EventOriginRotateHorizontal
  (params (value :type Float%20%28single-precision%29))
  (Transformation|AddRelativeRotation (Variables|Default|GetRotOrigin) (Math|Rotator|MakeRotator 0.0 0.0 value) false false))

(event EventTick
  (params (DeltaSeconds :type Float%20%28single-precision%29))
  (bind _camera (Variables|Default|GetCamera))
  (Transformation|SetRelativeLocation _camera (Math|Vector|Lerp(Vector) (Variables|/Script/Engine.SceneComponent|GetRelativeLocation _camera) (Variables|/Script/Engine.SceneComponent|GetRelativeLocation (Variables|Default|GetZoomTarget)) (* DeltaSeconds (Variables|Default|GetZoomSpeed))) false false))

(event EventOriginRotateVertical
  (params (value :type Float%20%28single-precision%29))
  (bind _rotorigin (Variables|Default|GetRotOrigin))
  (bind _relativerotation (Variables|/Script/Engine.SceneComponent|GetRelativeRotation _rotorigin))
  (bind (_roll _pitch _yaw) (Math|Rotator|BreakRotator _relativerotation))
  (Transformation|SetRelativeRotation _rotorigin (Math|Rotator|MakeRotator _roll (Math|Float|Clamp(Float) (+ value _pitch) (Variables|Default|GetMinPitch) (Variables|Default|GetMaxPitch)) _yaw) false false))

(event EventZoomTargetZoom
  (params (value :type Float%20%28single-precision%29))
  (bind _zoomtarget (Variables|Default|GetZoomTarget))
  (Transformation|SetRelativeLocation _zoomtarget (Math|Vector|MakeVector (* (Math|Float|Clamp(Float) (Math|Vector|Distance(Vector) (+ value (Variables|/Script/Engine.SceneComponent|GetRelativeLocation _zoomtarget)) "0, 0, 0") (Variables|Default|GetMinZoom) (Variables|Default|GetMaxZoom)) -1.0) 0.0 0.0) false false))

(fn ConstructionScript
  (Variables|Default|SetMinPitch -4e+01)
  (Variables|Default|SetMaxPitch -5.0)
  (Variables|Default|SetZoomSpeed 5.0)
  (Variables|Default|SetCameraOriginSpawnLocation "0, 0,100.000000")
  (Variables|Default|SetMinZoom 3.5e+02)
  (Variables|Default|SetMaxZoom 2e+03))