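; Trigger actor that punches a mesh forward to set off a referenced wall, apparently for a wall destruction animation.
; The mesh starts hidden; any Box overlap reveals it and plays the Punch timeline, lerping it from its starting relative position to local zero.
; While the track exceeds 0.9, each update calls the wall's animation event, so it can fire repeatedly.
; The mesh hides again when the timeline finishes.
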(event OnComponentBeginOverlap(Box)
  (params (OverlappedComponent :type Primitive%20Component%20Object%20Reference) (OtherActor :type Actor%20Object%20Reference) (OtherComp :type Primitive%20Component%20Object%20Reference) (OtherBodyIndex :type Integer) (bFromSweep :type Boolean) (SweepResult :type Hit%20Result%20Structure%20%28by%20ref%29))
  (bind _staticmesh (Variables|Default|GetStaticMesh))
  (Rendering|SetVisibility _staticmesh true false)
  (bind _newtrack_0 (Timeline|punch Play)
    (:Update
      (Transformation|SetRelativeLocation _staticmesh (Math|Vector|Lerp(Vector) (Variables|Default|GetstartingPos) (Math|Vector|MakeVector 0.0 0.0 0.0) _newtrack_0) false false)
      (if (> _newtrack_0 0.9)
        (Default|HasAnimatedEvntEvent (Variables|Default|Getwall))))
    (:Finished
      (Rendering|SetVisibility _staticmesh false false))))

(event EventBeginPlay
  (bind _staticmesh (Variables|Default|GetStaticMesh))
  (Variables|Default|SetstartingPos (Variables|/Script/Engine.SceneComponent|GetRelativeLocation _staticmesh))
  (Rendering|SetVisibility _staticmesh false false))

(fn ConstructionScript)