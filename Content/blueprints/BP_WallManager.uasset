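; BP_WallManager is a wall Blueprint that switches between a full and a cut mesh, as in a wall cutaway view.
; The construction script adds the static mesh component stored as CurrentWall, which BeginPlay sets to FullWall.
; ChangeState_Event swaps it to FullWall or CutWall based on IsUp, only while HasAnimated is false; nothing shown here sets that flag.
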(event Custom|ChangeState_Event
  (params (isUp :type Boolean))
  (bind _currentwall (Variables|Default|GetCurrentWall))
  (if (not (Variables|Default|GethasAnimated))
    (if isUp
      (Components|StaticMesh|SetStaticMesh _currentwall (Variables|Default|GetfullWall))
      (else
        (Components|StaticMesh|SetStaticMesh _currentwall (Variables|Default|GetcutWall))))))

(event EventBeginPlay
  (Components|StaticMesh|SetStaticMesh (Variables|Default|GetCurrentWall) (Variables|Default|GetfullWall)))

(fn ConstructionScript
  (bind _returnvalue (AddComponent|AddStaticMeshComponent false))
  (Variables|Default|SetCurrentWall _returnvalue))