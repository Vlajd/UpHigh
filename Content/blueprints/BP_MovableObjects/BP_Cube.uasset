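; BP_Cube is a movable box that the player character can push.
; Overlaps on its XCol and YCol volumes both call SetPushing, which acts only on BP_CharacterController actors.
; SetPushing enables physics simulation on the box and sets IsCharacterPushing on the character's anim instance when overlap begins, and clears both when it ends.
; The two volumes share this state without overlap counting, so leaving either one switches pushing off.
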(event OnComponentBeginOverlap(XCol)
  (params (OverlappedComponent :type Primitive%20Component%20Object%20Reference) (OtherActor :type Actor%20Object%20Reference) (OtherComp :type Primitive%20Component%20Object%20Reference) (OtherBodyIndex :type Integer) (bFromSweep :type Boolean) (SweepResult :type Hit%20Result%20Structure%20%28by%20ref%29))
  (CallFunction|SetPushing OtherActor true (Variables|Default|GetBox)))

(event OnComponentBeginOverlap(YCol)
  (params (OverlappedComponent :type Primitive%20Component%20Object%20Reference) (OtherActor :type Actor%20Object%20Reference) (OtherComp :type Primitive%20Component%20Object%20Reference) (OtherBodyIndex :type Integer) (bFromSweep :type Boolean) (SweepResult :type Hit%20Result%20Structure%20%28by%20ref%29))
  (CallFunction|SetPushing OtherActor true (Variables|Default|GetBox)))

(event OnComponentEndOverlap(XCol)
  (params (OverlappedComponent :type Primitive%20Component%20Object%20Reference) (OtherActor :type Actor%20Object%20Reference) (OtherComp :type Primitive%20Component%20Object%20Reference) (OtherBodyIndex :type Integer))
  (CallFunction|SetPushing OtherActor false (Variables|Default|GetBox)))

(event OnComponentEndOverlap(YCol)
  (params (OverlappedComponent :type Primitive%20Component%20Object%20Reference) (OtherActor :type Actor%20Object%20Reference) (OtherComp :type Primitive%20Component%20Object%20Reference) (OtherBodyIndex :type Integer))
  (CallFunction|SetPushing OtherActor false (Variables|Default|GetBox)))

(fn ConstructionScript)

(fn SetPushing
  (params (Other :type Actor%20Object%20Reference) (SetBools :type Boolean) (WhichCube :type Static%20Mesh%20Component%20Object%20Reference%20%28by%20ref%29))
  (bind _asbp_character_controller (Utilities|Casting|CastToBP_CharacterController Other))
  (Physics|SetSimulatePhysics WhichCube SetBools)
  (bind _asbp_character_anim (Utilities|Casting|CastToBP_Character_Anim (Components|SkeletalMesh|GetAnimInstance (Variables|/Game/blueprints/BP_CharacterController.BP_CharacterController_C|GetCharacterSkeletalMesh _asbp_character_controller))))
  (Variables|/Game/blueprints/BP_Character_Anim.BP_Character_Anim_C|SetIsCharacterPushing _asbp_character_anim SetBools))